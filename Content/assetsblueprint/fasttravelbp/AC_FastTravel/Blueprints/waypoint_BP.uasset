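; Fast travel waypoint actor that becomes discovered when the player reaches it and opens a waypoint menu.
; Box overlap with MyFps draws an interaction prompt and sets the discovered flag; leaving removes the prompt.
; Pressing F removes the prompt, then shows Waypoint_widget with UI-only input and a mouse cursor.
; The construction script caches the static mesh's world location as WayPointLocation.
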(event `self.Box.OnComponentBeginOverlap`
  (params (OverlappedComponent :type "PrimitiveComponent Object Reference") (OtherActor :type "Actor Object Reference") (OtherComp :type "PrimitiveComponent Object Reference") (OtherBodyIndex :type Integer) (bFromSweep :type Boolean) (SweepResult :type "HitResult Structure (by ref)"))
  (cast `/Game/Migrate/MyFps` OtherActor)
  (`/Game/assetsblueprint/fasttravelbp/AC_FastTravel/Macro/M_interaction.DrawInteractionWidget` self (`self.InteractionText`)
    (:`NewParam`
      (`self.Check Discovered`))))

(event `self.Box.OnComponentEndOverlap`
  (params (OverlappedComponent :type "PrimitiveComponent Object Reference") (OtherActor :type "Actor Object Reference") (OtherComp :type "PrimitiveComponent Object Reference") (OtherBodyIndex :type Integer))
  (cast `/Game/Migrate/MyFps` OtherActor)
  (`/Game/assetsblueprint/fasttravelbp/AC_FastTravel/Macro/M_interaction.RemoveInteractionWidget` self))

(event `Key|F`
  (params (Key :type "Key Structure"))
  (:`Pressed`
    (`/Game/assetsblueprint/fasttravelbp/AC_FastTravel/Macro/M_interaction.RemoveInteractionWidget` self
      (:`NewParam`
        (`self.ShowWaypointWidget`)))))

(fn `Check Discovered`
  (if (not (`self.Hasdiscorvered`))
    (set `self.Hasdiscorvered` true)))

(fn `ShowWaypointWidget`
  (bind _returnvalue (`GameplayStatics.GetPlayerController` 0))
  (bind _returnvalue_2 (`|CreateWidget` "/Game/assetsblueprint/fasttravelbp/AC_FastTravel/widget/waypoint_widget.waypoint_widget_C"))
  (`UserWidget.AddToViewport` _returnvalue_2 0)
  (`WidgetBlueprintLibrary.SetInputMode_UIOnlyEx` _returnvalue _returnvalue_2)
  (set `PlayerController.bShowMouseCursor` true _returnvalue))

(fn `UserConstructionScript`
  (set `self.WayPointLocation` (`SceneComponent.K2_GetComponentLocation` (`self.StaticMesh`))))